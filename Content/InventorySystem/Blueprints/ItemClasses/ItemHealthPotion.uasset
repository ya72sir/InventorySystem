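; Health potion item class for the inventory system that restores a fixed amount of health to the top-down character when used.
; On use, it checks current HP against max through the Inventory's character reference, then heals and removes one item from its inventory index.
; At full health it leaves the inventory untouched; the actor destroys itself in either case.
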(event EventBeginPlay
  (|CallParentFunction) ; This node is disabled and will not be called.\nDrag off pins to build functionality.
)

(event Collision|EventActorBeginOverlap
  (params (OtherActor :type Actor%20Object%20Reference))
  (|CallParentFunction OtherActor) ; This node is disabled and will not be called.\nDrag off pins to build functionality.
)

(event EventTick
  (params (DeltaSeconds :type Float%20%28single-precision%29))
  (|CallParentFunction DeltaSeconds) ; This node is disabled and will not be called.\nDrag off pins to build functionality.
)

(event EventEventonUsed
  (bind _inventory (Variables|Default|GetInventory))
  (bind _topdowncharref (Variables|/Game/InventorySystem/Blueprints/bp_Inventory.bp_Inventory_C|GetTopDownCharRef _inventory))
  (if (< (Variables|/Game/TopDownBP/Blueprints/TopDownCharacter.TopDownCharacter_C|GetCurrentHP _topdowncharref) (Variables|/Game/TopDownBP/Blueprints/TopDownCharacter.TopDownCharacter_C|GetMaxHP _topdowncharref))
    (Default|-IncreaseHealth _topdowncharref 10)
    (Default|-RemoveItematIndex (Variables|Default|GetInventory) (Variables|Default|GetIndex) 1 false)
    (Actor|DestroyActor)
    (else
      (Actor|DestroyActor))))

(fn ConstructionScript
  (|CallParentFunction))