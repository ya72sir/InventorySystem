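; Inventory map item that shows an old map on screen when used and is consumed once read.
; On use, it disables the inventory widget, adds a centered W_OldMap to the main widget canvas with a reference to itself, and switches input to UI only.
; OnRead removes the map, re-enables the inventory, restores game-and-UI input and destroys the item actor.
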(event Custom|OnRead
  (Widget|SetIsEnabled (Variables|/Game/InventorySystem/Widgets/w_MainWidget.w_MainWidget_C|GetInventoryWidget (Variables|/Game/InventorySystem/Blueprints/bp_Inventory.bp_Inventory_C|GetMainWidget (Variables|Default|GetInventory))) true)
  (Widget|RemovefromParent (Variables|Default|GetMapWidget))
  (Input|SetInputModeGameandUI (Game|GetPlayerController 0) 0 "DoNotLock" false)
  (Actor|DestroyActor))

(event EventBeginPlay
  (|CallParentFunction) ; This node is disabled and will not be called.\nDrag off pins to build functionality.
)

(event Collision|EventActorBeginOverlap
  (params (OtherActor :type Actor%20Object%20Reference))
  (|CallParentFunction OtherActor) ; This node is disabled and will not be called.\nDrag off pins to build functionality.
)

(event EventTick
  (params (DeltaSeconds :type Float%20%28single-precision%29))
  (|CallParentFunction DeltaSeconds) ; This node is disabled and will not be called.\nDrag off pins to build functionality.
)

(event EventEventonUsed
  (Widget|SetIsEnabled (Variables|/Game/InventorySystem/Widgets/w_MainWidget.w_MainWidget_C|GetInventoryWidget (Variables|/Game/InventorySystem/Blueprints/bp_Inventory.bp_Inventory_C|GetMainWidget (Variables|Default|GetInventory))) false)
  (bind _returnvalue (UserInterface|CreateWidget "/Game/InventorySystem/Widgets/w_OldMap.w_OldMap_C" 0 self))
  (bind _output_get (Variables|Default|SetMapWidget _returnvalue))
  (bind _returnvalue_2 (Class|CanvasPanel|AddChildtoCanvas (Variables|/Game/InventorySystem/Widgets/w_MainWidget.w_MainWidget_C|GetCanvas (Variables|/Game/InventorySystem/Blueprints/bp_Inventory.bp_Inventory_C|GetMainWidget (Variables|Default|GetInventory))) _output_get))
  (Class|CanvasPanelSlot|SetAnchors _returnvalue_2 (Utilities|Struct|MakeAnchors "(X=0.500000,Y=0.500000)" "(X=0.500000,Y=0.500000)"))
  (Class|CanvasPanelSlot|SetAutoSize _returnvalue_2 true)
  (Class|CanvasPanelSlot|SetAlignment _returnvalue_2 "(X=0.500000,Y=0.500000)")
  (Input|SetInputModeUIOnly (Game|GetPlayerController 0) (Variables|Default|GetMapWidget) "DoNotLock"))

(fn ConstructionScript
  (|CallParentFunction))