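; Interactable world map point that lets the top-down character open the map screen from the inventory UI.
; A sphere overlap registers this actor as the character's MarkMap and shows a "Press [E]" prompt, reusing the merchant text widget; leaving clears both.
; OnInteract shows the WMaps widget, switches input to UI-only, hands it the character and calls CurrentMap.
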(event OnComponentBeginOverlap(Sphere)
  (params (OverlappedComponent :type Primitive%20Component%20Object%20Reference) (OtherActor :type Actor%20Object%20Reference) (OtherComp :type Primitive%20Component%20Object%20Reference) (OtherBodyIndex :type Integer) (bFromSweep :type Boolean) (SweepResult :type Hit%20Result%20Structure%20%28by%20ref%29))
  (bind _astop_down_character (Utilities|Casting|CastToTopDownCharacter OtherActor))
  (bind _output_get (Variables|Default|SetTopDownCharacter _astop_down_character))
  (Variables|/Game/TopDownBP/Blueprints/TopDownCharacter.TopDownCharacter_C|SetMarkMap _output_get self)
  (Rendering|SetVisibility (Variables|Default|GetWidget) true false))

(event OnComponentEndOverlap(Sphere)
  (params (OverlappedComponent :type Primitive%20Component%20Object%20Reference) (OtherActor :type Actor%20Object%20Reference) (OtherComp :type Primitive%20Component%20Object%20Reference) (OtherBodyIndex :type Integer))
  (bind _astop_down_character (Utilities|Casting|CastToTopDownCharacter OtherActor))
  (Variables|/Game/TopDownBP/Blueprints/TopDownCharacter.TopDownCharacter_C|SetMarkMap _astop_down_character 0)
  (Rendering|SetVisibility (Variables|Default|GetWidget) false false))

(event Custom|OnInteract
  (bind _topdowncharacter (Variables|Default|GetTopDownCharacter))
  (bind _inventoryref (Variables|/Game/TopDownBP/Blueprints/TopDownCharacter.TopDownCharacter_C|GetInventoryRef _topdowncharacter))
  (bind _mainwidget (Variables|/Game/InventorySystem/Blueprints/bp_Inventory.bp_Inventory_C|GetMainWidget _inventoryref))
  (bind _w_maps (Variables|/Game/InventorySystem/Widgets/w_MainWidget.w_MainWidget_C|Getw_Maps _mainwidget))
  (Variables|Default|SetIsOpen? true)
  (Widget|SetVisibility _w_maps "Visible")
  (Input|SetInputModeUIOnly (Game|GetPlayerController 0) _w_maps "DoNotLock")
  (Variables|/Game/InventorySystem/Widgets/w_Maps.w_Maps_C|SetTopDownCharater _w_maps (Variables|Default|GetTopDownCharacter))
  (Default|-CurrentMap _w_maps))

(event EventBeginPlay
  (bind _asw_merchant_text (Utilities|Casting|CastTow_MerchantText (UserInterface|GetUserWidgetObject (Variables|Default|GetWidget))))
  (Default|-SetText _asw_merchant_text "World" "Press [E] to open the map"))

(fn ConstructionScript)