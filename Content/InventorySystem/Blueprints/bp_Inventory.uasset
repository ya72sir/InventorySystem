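; Slot-based inventory for the top-down character, which creates the main HUD widget and registers itself on the character.
; Slots store item class and amount, with item info read from class defaults and using an item spawning its actor.
; Adding recursively fills partial stacks, then empty slots, returning any remainder and optionally queuing an obtained message.
; Remove, swap, merge and split functions edit the array and refresh affected slot widgets.
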(event Custom|UpdateSlotAtIndex
  (params (Index :type Integer))
  (Default|UpdateSlot (Utilities|Array|Get(acopy) (Variables|/Game/InventorySystem/Widgets/w_Inventory.w_Inventory_C|GetSlotsWidgets (Variables|Default|GetInventoryWidget)) Index)))

(event Custom|UseItemAtIndex
  (params (Index :type Integer))
  (bind _slots (Variables|Default|GetSlots))
  (bind _output (Utilities|Array|Get(acopy) _slots Index))
  (bind _itemclass (Utilities|Struct|Breaks_InventorySlot _output))
  (if (Utilities|IsValidClass _itemclass)
    (bind _returnvalue (Game|SpawnActorfromClass _itemclass (Math|Transform|MakeTransform "0, 0, 0" "0, 0, 0" "1,1,1") "AlwaysSpawn" 0 self Index 0))
    (Default|EventonUsed _returnvalue)))

(event EventBeginPlay
  (Utilities|Array|Resize (Variables|Default|GetSlots) (Variables|Default|GetAmountOfSlots))
  (bind _returnvalue (UserInterface|CreateWidget "/Game/InventorySystem/Widgets/w_MainWidget.w_MainWidget_C" 0 self (Variables|Default|GetSlotsPerRow) (Variables|Default|GetObtainedVisibleDuration)))
  (bind _output_get (Variables|Default|SetMainWidget _returnvalue))
  (Variables|Default|SetInventoryWidget (Variables|/Game/InventorySystem/Widgets/w_MainWidget.w_MainWidget_C|GetInventoryWidget _output_get))
  (Default|-UpdateHealthBar (Variables|Default|GetTopDownCharRef))
  (UserInterface|Viewport|AddtoViewport (Variables|Default|GetMainWidget) 0)
  (if (not (Variables|Default|GetShowObtainedMessage?))
    (Widget|RemovefromParent (Variables|/Game/InventorySystem/Widgets/w_MainWidget.w_MainWidget_C|GetObtainedItemBorder (Variables|Default|GetMainWidget)))))

(fn ConstructionScript
  (Variables|/Game/TopDownBP/Blueprints/TopDownCharacter.TopDownCharacter_C|SetInventoryRef (Variables|Default|GetTopDownCharRef) self))

(fn -IsSlotEmpty?
  (params (Index :type Integer))
  (return (not (Utilities|IsValidClass (.ItemClass (Utilities|Struct|Breaks_InventorySlot (Utilities|Array|Get(acopy) (Variables|Default|GetSlots) Index)))))))

(fn -GetItemInfoatIndex
  (params (Index :type Integer))
  (bind _slots (Variables|Default|GetSlots))
  (bind _output (Utilities|Array|Get(acopy) _slots Index))
  (bind (_itemclass _amount) (Utilities|Struct|Breaks_InventorySlot _output))
  (if (Utilities|IsValidClass _itemclass)
    (return false (.ItemInfo (Utilities|GetClassDefaults _itemclass)) _amount)
    (else
      (return true "" 0))))

(fn -SearchEmptySlot
  (bind (_array_element _array_index) (Utilities|Array|ForEachLoopwithBreak (Variables|Default|GetSlots) :!label _label)
    (:LoopBody
      (if (not (Utilities|IsValidClass (.ItemClass (Utilities|Struct|Breaks_InventorySlot _array_element))))
        (LocalVariables|Setlocal_Bool true)
        (LocalVariables|SetLocalIndex _array_index)
        (goto _label Break)))
    (:Completed
      (return (LocalVariables|Getlocal_Bool) (LocalVariables|GetLocalIndex)))))

(fn -SearchFreeStack
  (params (ItemClass :type Bp%20Master%20Item%20Class%20Reference))
  (bind (_array_element _array_index) (Utilities|Array|ForEachLoopwithBreak (Variables|Default|GetSlots) :!label _label)
    (:LoopBody
      (if (Utilities|IsValidClass (.ItemClass (Utilities|Struct|Breaks_InventorySlot _array_element)))
        (if (and (== (.ItemClass (Utilities|Struct|Breaks_InventorySlot _array_element)) ItemClass) (< (.Amount (Utilities|Struct|Breaks_InventorySlot _array_element)) (Variables|Default|GetMaxStackSize)))
          (LocalVariables|Setlocal_Bool true)
          (LocalVariables|Setlocal_Index _array_index)
          (goto _label Break))))
    (:Completed
      (return (LocalVariables|Getlocal_Bool) (LocalVariables|Getlocal_Index)))))

(fn -AddItem
  (params (ItemClass :type Bp%20Master%20Item%20Class%20Reference) (Amount :type Integer))
  (if (Variables|Default|GetShowObtainedMessage?)
    (bind (_success_ _rest) (CallFunction|-AddItem(Internal) ItemClass Amount))
    (if _success_
      (CallFunction|-ShowObtainedItem ItemClass (- Amount _rest))
      (return true _rest)
      (else
        (return false _rest)))
    (else
      (bind (_success__2 _rest_2) (CallFunction|-AddItem(Internal) ItemClass Amount))
      (return _success__2 _rest_2))))

(fn -GetAmountatIndex
  (params (Index :type Integer))
  (return (.Amount (Utilities|Struct|Breaks_InventorySlot (Utilities|Array|Get(acopy) (Variables|Default|GetSlots) Index)))))

(fn -ShowInvetory
  (Widget|SetVisibility (Variables|Default|GetInventoryWidget) "Visible")
  (Variables|Default|SetisVisible? true)
  (Widget|SetIsEnabled (Variables|Default|GetInventoryWidget) true)
  (return))

(fn -HideInvetory
  (Widget|SetVisibility (Variables|Default|GetInventoryWidget) "Hidden")
  (Variables|Default|SetisVisible? false)
  (Widget|SetIsEnabled (Variables|Default|GetInventoryWidget) false)
  (Widget|SetVisibility (Variables|/Game/InventorySystem/Widgets/w_MainWidget.w_MainWidget_C|GetThrowAwayWidget (Variables|Default|GetMainWidget)) "Hidden")
  (Widget|SetIsEnabled (Variables|/Game/InventorySystem/Widgets/w_Inventory.w_Inventory_C|GetSlotPanel (Variables|Default|GetInventoryWidget)) true)
  (return))

(fn -RemoveItematIndex
  (params (Index :type Integer) (Amount :type Integer))
  (bind _slots (Variables|Default|GetSlots))
  (LocalVariables|Setlocal_Index Index)
  (LocalVariables|Setlocal_Amount Amount)
  (if (and (not (CallFunction|-IsSlotEmpty? (LocalVariables|Getlocal_Index))) (> (LocalVariables|Getlocal_Amount) 0))
    (if (>= (LocalVariables|Getlocal_Amount) (CallFunction|-GetAmountatIndex (LocalVariables|Getlocal_Index)))
      (Utilities|Array|SetArrayElem (Variables|Default|GetSlots) (LocalVariables|Getlocal_Index) (Utilities|Struct|Makes_InventorySlot 0 0))
      (CallFunction|UpdateSlotatIndex (LocalVariables|Getlocal_Index))
      (return true)
      (else
        (Utilities|Array|SetArrayElem _slots (LocalVariables|Getlocal_Index) (Utilities|Struct|Makes_InventorySlot (.itemclass (Utilities|Array|Get(acopy) _slots (LocalVariables|Getlocal_Index))) (- (.amount (Utilities|Array|Get(acopy) _slots (LocalVariables|Getlocal_Index))) (LocalVariables|Getlocal_Amount))))
        (CallFunction|UpdateSlotatIndex (LocalVariables|Getlocal_Index))
        (return true)))
    (else
      (return false))))

(fn -SwapSlots
  (params (Index1 :type Integer) (Index2 :type Integer))
  (bind _slots (Variables|Default|GetSlots))
  (bind _slots_2 (Variables|Default|GetSlots))
  (bind _returnvalue (Utilities|Array|LastIndex _slots))
  (LocalVariables|Setlocal_Index1 Index1)
  (LocalVariables|Setlocal_Index2 Index2)
  (if (or (> (LocalVariables|Getlocal_Index1) _returnvalue) (> (LocalVariables|Getlocal_Index2) _returnvalue))
    (return false)
    (else
      (LocalVariables|Setlocal_Slot2 (Utilities|Array|Get(acopy) (Variables|Default|GetSlots) (LocalVariables|Getlocal_Index2)))
      (Utilities|Array|SetArrayElem _slots_2 (LocalVariables|Getlocal_Index2) (Utilities|Array|Get(acopy) _slots_2 (LocalVariables|Getlocal_Index1)))
      (Utilities|Array|SetArrayElem (Variables|Default|GetSlots) (LocalVariables|Getlocal_Index1) (LocalVariables|Getlocal_Slot2))
      (CallFunction|UpdateSlotatIndex (LocalVariables|Getlocal_Index1))
      (CallFunction|UpdateSlotatIndex (LocalVariables|Getlocal_Index2))
      (return true))))

(fn -SplitStack
  (params (StackIndex :type Integer) (Amount :type Integer))
  (bind _slots (Variables|Default|GetSlots))
  (bind _slots_2 (Variables|Default|GetSlots))
  (LocalVariables|Setlocal_StackIndex StackIndex)
  (LocalVariables|Setlocal_Amount Amount)
  (if (CallFunction|-IsSlotEmpty? (LocalVariables|Getlocal_StackIndex))
    (return false)
    (elif (and (.canBeStacked? (Utilities|Struct|Breaks_ItemInfo (.Item%20Info (CallFunction|-GetItemInfoatIndex (LocalVariables|Getlocal_StackIndex))))) (> (.Amount (CallFunction|-GetItemInfoatIndex (LocalVariables|Getlocal_StackIndex))) (LocalVariables|Getlocal_Amount)))
      (bind (_success_ _index) (CallFunction|-SearchEmptySlot))
      (if _success_
        (LocalVariables|Setlocal_FoundIndex _index)
        (Utilities|Array|SetArrayElem _slots_2 (LocalVariables|Getlocal_StackIndex) (Utilities|Struct|Makes_InventorySlot (.itemclass (Utilities|Array|Get(acopy) _slots_2 (LocalVariables|Getlocal_StackIndex))) (- (.amount (Utilities|Array|Get(acopy) _slots_2 (LocalVariables|Getlocal_StackIndex))) (LocalVariables|Getlocal_Amount))))
        (Utilities|Array|SetArrayElem _slots (LocalVariables|Getlocal_FoundIndex) (Utilities|Struct|Makes_InventorySlot (.itemclass (Utilities|Array|Get(acopy) _slots (LocalVariables|Getlocal_StackIndex))) (LocalVariables|Getlocal_Amount)))
        (CallFunction|UpdateSlotatIndex (LocalVariables|Getlocal_StackIndex))
        (CallFunction|UpdateSlotatIndex (LocalVariables|Getlocal_FoundIndex))
        (return true)
        (else
          (return false)))
      (else
        (return false)))))

(fn -AddtoIndex
  (params (FromIndex :type Integer) (ToIndex :type Integer))
  (LocalVariables|Setlocal_From FromIndex)
  (LocalVariables|Setlocal_To ToIndex)
  (if (Math|Boolean|ANDBoolean (== (.itemclass (Utilities|Array|Get(acopy) (Variables|Default|GetSlots) (LocalVariables|Getlocal_From))) (.itemclass (Utilities|Array|Get(acopy) (Variables|Default|GetSlots) (LocalVariables|Getlocal_To)))) (< (.amount (Utilities|Array|Get(acopy) (Variables|Default|GetSlots) (LocalVariables|Getlocal_To))) (Variables|Default|GetMaxStackSize)) (.canBeStacked? (Utilities|Struct|Breaks_ItemInfo (.Item%20Info (CallFunction|-GetItemInfoatIndex (LocalVariables|Getlocal_From))))))
    (LocalVariables|Setlocal_Class (.itemclass (Utilities|Array|Get(acopy) (Variables|Default|GetSlots) (LocalVariables|Getlocal_From))))
    (if (>= (- (Variables|Default|GetMaxStackSize) (CallFunction|-GetAmountatIndex (LocalVariables|Getlocal_To))) (CallFunction|-GetAmountatIndex (LocalVariables|Getlocal_From)))
      (Utilities|Array|SetArrayElem (Variables|Default|GetSlots) (LocalVariables|Getlocal_To) (Utilities|Struct|Makes_InventorySlot (LocalVariables|Getlocal_Class) (+ (CallFunction|-GetAmountatIndex (LocalVariables|Getlocal_From)) (CallFunction|-GetAmountatIndex (LocalVariables|Getlocal_To)))))
      (Utilities|Array|SetArrayElem (Variables|Default|GetSlots) (LocalVariables|Getlocal_From) (Utilities|Struct|Makes_InventorySlot 0 0))
      (else
        (Utilities|Array|SetArrayElem (Variables|Default|GetSlots) (LocalVariables|Getlocal_From) (Utilities|Struct|Makes_InventorySlot (LocalVariables|Getlocal_Class) (- (CallFunction|-GetAmountatIndex (LocalVariables|Getlocal_From)) (- (Variables|Default|GetMaxStackSize) (CallFunction|-GetAmountatIndex (LocalVariables|Getlocal_To))))))
        (Utilities|Array|SetArrayElem (Variables|Default|GetSlots) (LocalVariables|Getlocal_To) (Utilities|Struct|Makes_InventorySlot (LocalVariables|Getlocal_Class) (Variables|Default|GetMaxStackSize)))))
    (CallFunction|UpdateSlotatIndex (LocalVariables|Getlocal_From))
    (CallFunction|UpdateSlotatIndex (LocalVariables|Getlocal_To))
    (return true)
    (else
      (return false))))

(fn -SplitStacktoIndex
  (params (FromIndex :type Integer) (ToIndex :type Integer) (Amount :type Integer))
  (LocalVariables|Setlocal_From FromIndex)
  (LocalVariables|Setlocal_To ToIndex)
  (LocalVariables|Setlocal_Amount Amount)
  (if (Math|Boolean|ANDBoolean (CallFunction|-IsSlotEmpty? (LocalVariables|Getlocal_To)) (not (CallFunction|-IsSlotEmpty? (LocalVariables|Getlocal_From))) (.canBeStacked? (Utilities|Struct|Breaks_ItemInfo (.Item%20Info (CallFunction|-GetItemInfoatIndex (LocalVariables|Getlocal_From))))) (> (.Amount (CallFunction|-GetItemInfoatIndex (LocalVariables|Getlocal_From))) 1) (> (.Amount (CallFunction|-GetItemInfoatIndex (LocalVariables|Getlocal_From))) (LocalVariables|Getlocal_Amount)))
    (LocalVariables|Setlocal_Class (.itemclass (Utilities|Array|Get(acopy) (Variables|Default|GetSlots) (LocalVariables|Getlocal_From))))
    (Utilities|Array|SetArrayElem (Variables|Default|GetSlots) (LocalVariables|Getlocal_From) (Utilities|Struct|Makes_InventorySlot (LocalVariables|Getlocal_Class) (- (.amount (Utilities|Array|Get(acopy) (Variables|Default|GetSlots) (LocalVariables|Getlocal_From))) (LocalVariables|Getlocal_Amount))))
    (Utilities|Array|SetArrayElem (Variables|Default|GetSlots) (LocalVariables|Getlocal_To) (Utilities|Struct|Makes_InventorySlot (LocalVariables|Getlocal_Class) (LocalVariables|Getlocal_Amount)))
    (CallFunction|UpdateSlotatIndex (LocalVariables|Getlocal_From))
    (CallFunction|UpdateSlotatIndex (LocalVariables|Getlocal_To))
    (return true)
    (else
      (return false))))

(fn -ShowObtainedItem
  (params (ItemClass :type Bp%20Master%20Item%20Class%20Reference) (Amount :type Integer))
  (bind _mainwidget (Variables|Default|GetMainWidget))
  (if (Variables|Default|GetShowObtainedMessage?)
    (Utilities|IsValid _mainwidget
      (:Is%20Valid
        (Default|-AddItemtoObtainedQueue _mainwidget ItemClass Amount)
        (return true))
      (:Is%20Not%20Valid
        _)))
  (return false))

(fn -AddItem(Internal)
  (params (ItemClass :type Bp%20Master%20Item%20Class%20Reference) (Amount :type Integer))
  (bind _slots (Variables|Default|GetSlots))
  (LocalVariables|Setlocal_ItemClass ItemClass)
  (LocalVariables|Setlocal_Amount Amount)
  (if (.canBeStacked? (Utilities|Struct|Breaks_ItemInfo (.ItemInfo (Utilities|GetClassDefaults ItemClass))))
    (bind (_success_ _index) (CallFunction|-SearchFreeStack (LocalVariables|Getlocal_ItemClass)))
    (if _success_
      (LocalVariables|Setlocal_FoundIndex _index)
      (if (> (+ (.Amount (Utilities|Struct|Breaks_InventorySlot (Utilities|Array|Get(acopy) (Variables|Default|GetSlots) (LocalVariables|Getlocal_FoundIndex)))) (LocalVariables|Getlocal_Amount)) (Variables|Default|GetMaxStackSize))
        (LocalVariables|Setlocal_Amount (- (+ (.Amount (Utilities|Struct|Breaks_InventorySlot (Utilities|Array|Get(acopy) (Variables|Default|GetSlots) (LocalVariables|Getlocal_FoundIndex)))) (LocalVariables|Getlocal_Amount)) (Variables|Default|GetMaxStackSize)))
        (Utilities|Array|SetArrayElem _slots (LocalVariables|Getlocal_FoundIndex) (Utilities|Struct|Makes_InventorySlot (LocalVariables|Getlocal_ItemClass) (Variables|Default|GetMaxStackSize)))
        (CallFunction|UpdateSlotatIndex (LocalVariables|Getlocal_FoundIndex))
        (bind (_success__2 _rest) (CallFunction|-AddItem(Internal) (LocalVariables|Getlocal_ItemClass) (LocalVariables|Getlocal_Amount)))
        (return _success__2 _rest)
        (else
          (Utilities|Array|SetArrayElem _slots (LocalVariables|Getlocal_FoundIndex) (Utilities|Struct|Makes_InventorySlot (LocalVariables|Getlocal_ItemClass) (+ (.Amount (Utilities|Struct|Breaks_InventorySlot (Utilities|Array|Get(acopy) (Variables|Default|GetSlots) (LocalVariables|Getlocal_FoundIndex)))) (LocalVariables|Getlocal_Amount))))
          (CallFunction|UpdateSlotatIndex (LocalVariables|Getlocal_FoundIndex))
          (return true 0)))
      (else
        (bind (_success__3 _index_2) (CallFunction|-SearchEmptySlot))
        (if _success__3
          (bind _output_get (LocalVariables|Setlocal_FoundIndex _index_2))
          (if (> (LocalVariables|Getlocal_Amount) (Variables|Default|GetMaxStackSize))
            (Utilities|Array|SetArrayElem (Variables|Default|GetSlots) _output_get (Utilities|Struct|Makes_InventorySlot (LocalVariables|Getlocal_ItemClass) (Variables|Default|GetMaxStackSize)))
            (CallFunction|UpdateSlotatIndex (LocalVariables|Getlocal_FoundIndex))
            (bind (_success__4 _rest_2) (CallFunction|-AddItem(Internal) (LocalVariables|Getlocal_ItemClass) (- (LocalVariables|Getlocal_Amount) (Variables|Default|GetMaxStackSize))))
            (return _success__4 _rest_2)
            (else
              (Utilities|Array|SetArrayElem (Variables|Default|GetSlots) (LocalVariables|Getlocal_FoundIndex) (Utilities|Struct|Makes_InventorySlot (LocalVariables|Getlocal_ItemClass) (LocalVariables|Getlocal_Amount)))
              (CallFunction|UpdateSlotatIndex (LocalVariables|Getlocal_FoundIndex))
              (return true 0)))
          (else
            (return false (LocalVariables|Getlocal_Amount))))))
    (else
      (bind (_success__5 _index_3) (CallFunction|-SearchEmptySlot))
      (if _success__5
        (bind _output_get_2 (LocalVariables|Setlocal_FoundIndex _index_3))
        (Utilities|Array|SetArrayElem (Variables|Default|GetSlots) _output_get_2 (Utilities|Struct|Makes_InventorySlot (LocalVariables|Getlocal_ItemClass) 1))
        (CallFunction|UpdateSlotatIndex (LocalVariables|Getlocal_FoundIndex))
        (if (> (LocalVariables|Getlocal_Amount) 1)
          (bind (_success__6 _rest_3) (CallFunction|-AddItem(Internal) (LocalVariables|Getlocal_ItemClass) (- (LocalVariables|Getlocal_Amount) 1)))
          (return _success__6 _rest_3)
          (else
            (return true 0)))
        (else
          (return false (LocalVariables|Getlocal_Amount)))))))