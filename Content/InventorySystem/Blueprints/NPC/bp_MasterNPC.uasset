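; Base NPC Blueprint that acts as a merchant, with a chest actor serving as its shop stock.
; On BeginPlay it optionally rolls starter items from a data table by chance, converts the offer to stacked storage entries and spawns the chest with them.
; Interaction registers that chest with the player, and closing the shop restores walking and refreshes visible inventory.
; Cursor hover enables custom-depth highlighting with an enemy or NPC post-process volume.
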(event OnBeginCursorOver(CapsuleComponent)
  (params (TouchedComponent :type Primitive%20Component%20Object%20Reference))
  (bind _returnvalue (Game|GetPlayerCharacter 0))
  (bind _astop_down_character (Utilities|Casting|CastToTopDownCharacter _returnvalue))
  (Variables|/Script/Engine.PostProcessVolume|SetbEnabled (Variables|/Game/TopDownBP/Blueprints/TopDownCharacter.TopDownCharacter_C|GetPostProcessVolumeEnemy _astop_down_character) (Utilities|Enum|Equal(Enum) (Variables|Default|GetTypeNPC) "NewEnumerator0"))
  (Variables|/Script/Engine.PostProcessVolume|SetbEnabled (Variables|/Game/TopDownBP/Blueprints/TopDownCharacter.TopDownCharacter_C|GetPostProcessVolumeNPC _astop_down_character) (Utilities|Enum|Equal(Enum) (Variables|Default|GetTypeNPC) "NewEnumerator1"))
  (Rendering|SetRenderCustomDepth (Variables|Character|GetMesh) true))

(event OnEndCursorOver(CapsuleComponent)
  (params (TouchedComponent :type Primitive%20Component%20Object%20Reference))
  (bind _returnvalue (Game|GetPlayerCharacter 0))
  (bind _astop_down_character (Utilities|Casting|CastToTopDownCharacter _returnvalue))
  (Variables|/Script/Engine.PostProcessVolume|SetbEnabled (Variables|/Game/TopDownBP/Blueprints/TopDownCharacter.TopDownCharacter_C|GetPostProcessVolumeNPC _astop_down_character) false)
  (Variables|/Script/Engine.PostProcessVolume|SetbEnabled (Variables|/Game/TopDownBP/Blueprints/TopDownCharacter.TopDownCharacter_C|GetPostProcessVolumeEnemy _astop_down_character) false)
  (Rendering|SetRenderCustomDepth (Variables|Character|GetMesh) false))

(event Custom|OffInteract
  (Variables|Default|GetbpChest
    (:then
      (Variables|/Game/TopDownBP/Blueprints/TopDownCharacter.TopDownCharacter_C|SetNearbyChest (Variables|Default|GetTopDownChar) 0))
    (:else)))

(event Custom|OnInteract
  (params (TopDownCharacter :type Top%20Down%20Character%20Object%20Reference))
  (Variables|Default|SetTopDownChar TopDownCharacter)
  (bind _bpchest (Variables|Default|GetbpChest)
    (:then
      (Variables|/Game/TopDownBP/Blueprints/TopDownCharacter.TopDownCharacter_C|SetNearbyChest (Variables|Default|GetTopDownChar) _bpchest))
    (:else)))

(event Custom|OnShopClosed
  (bind _topdownchar (Variables|Default|GetTopDownChar))
  (bind _inventoryref (Variables|/Game/TopDownBP/Blueprints/TopDownCharacter.TopDownCharacter_C|GetInventoryRef _topdownchar))
  (Variables|/Game/TopDownBP/Blueprints/TopDownCharacter.TopDownCharacter_C|SetIsShopOpen? _topdownchar false)
  (Pawn|Components|CharacterMovement|SetMovementMode (Variables|/Script/Engine.Character|GetCharacterMovement _topdownchar) "MOVE_Walking" 0)
  (if (Variables|/Game/InventorySystem/Blueprints/bp_Inventory.bp_Inventory_C|GetisVisible? _inventoryref)
    (Default|-HideInvetory _inventoryref)
    (Default|-ShowInvetory _inventoryref)))

(event EventBeginPlay
  ;[1 0.1571 0.8597] BeginPlay
  (Utilities|FlowControl|Sequence
    (:then_0
      (if (Variables|Default|GetGenearteStartingItems?)
        (CallFunction|-GenerateStartingItems)))
    (:then_1
      (CallFunction|-GenerateStorageItems)
      (CallFunction|-AddChest))))

(fn ConstructionScript)

(fn -GenerateStartingItems
  (bind _outrownames (DataTable|GetDataTableRowNames "/Game/InventorySystem/Blueprints/DataTables/Table_MerchantStarterItems.Table_MerchantStarterItems"))
  (for _array_element _outrownames
    (bind _returnvalue (Utilities|GetDataTableRow "/Game/InventorySystem/Blueprints/DataTables/Table_MerchantStarterItems.Table_MerchantStarterItems" _array_element)
      (:then
        (if (Math|Boolean|ANDBoolean (Utilities|IsValidClass (.ItemClass (Utilities|Struct|Breaks_MerchantContent _returnvalue))) (>= (.Chance (Utilities|Struct|Breaks_MerchantContent _returnvalue)) (Math|Random|RandomIntegerinRange 1 100)) true)
          (Utilities|Array|Add (Variables|Default|GetOffer) (.ItemClass (Utilities|Struct|Breaks_MerchantContent _returnvalue))))))))

(fn -GenerateStorageItems
  (for _array_element (Variables|Default|GetOffer)
    (Utilities|Array|Add (Variables|Default|GetItemsStorage) (Utilities|Struct|Makes_InventorySlot _array_element (Math|Integer|SelectInt 25 1 (.canBeStacked? (Utilities|Struct|Breaks_ItemInfo (.ItemInfo (Utilities|GetClassDefaults _array_element))))))))
  (return))

(fn -AddChest
  (bind _self self)
  (bind _returnvalue (Game|SpawnActorfromClass "/Game/InventorySystem/Blueprints/bp_Chest.bp_Chest_C" (Math|Transform|MakeTransform "0, 0, 0" "0, 0, 0" "1,1,1") "Undefined" _self 20 5 (Variables|Default|GetItemsStorage) false _self))
  (bind _output_get (Variables|Default|SetbpChest _returnvalue))
  (Variables|/Game/InventorySystem/Blueprints/bp_Chest.bp_Chest_C|SetNPC _output_get self))