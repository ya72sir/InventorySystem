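; Enemy NPC that dies as soon as the TopDownCharacter overlaps its Interact component, turning the mesh into a physics body and disabling capsule collision.
; Hovering the capsule shows a resize left-right cursor.
; Once dead, hovering the mesh shows a closed-hand grab cursor and highlights the body through custom depth and the player character's enemy post-process volume, both switched off when the cursor leaves.
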(event OnBeginCursorOver(CapsuleComponent)
  (params (TouchedComponent :type Primitive%20Component%20Object%20Reference))
  (Variables|/Script/Engine.PlayerController|SetCurrentMouseCursor (Game|GetPlayerController 0) "ResizeLeftRight"))

(event OnEndCursorOver(CapsuleComponent)
  (params (TouchedComponent :type Primitive%20Component%20Object%20Reference))
  (Variables|/Script/Engine.PlayerController|SetCurrentMouseCursor (Game|GetPlayerController 0) "Default"))

(event OnComponentBeginOverlap(Interact)
  (params (OverlappedComponent :type Primitive%20Component%20Object%20Reference) (OtherActor :type Actor%20Object%20Reference) (OtherComp :type Primitive%20Component%20Object%20Reference) (OtherBodyIndex :type Integer) (bFromSweep :type Boolean) (SweepResult :type Hit%20Result%20Structure%20%28by%20ref%29))
  (Utilities|Casting|CastToTopDownCharacter OtherActor)
  (Physics|SetSimulatePhysics (Variables|Character|GetMesh) true)
  (Collision|SetCollisionEnabled (Variables|Default|GetCapsuleComponent) "NoCollision")
  (Variables|Default|SetisDeath? true))

(event OnBeginCursorOver(Mesh)
  (params (TouchedComponent :type Primitive%20Component%20Object%20Reference))
  (if (Variables|Default|GetisDeath?)
    (Variables|/Script/Engine.PlayerController|SetCurrentMouseCursor (Game|GetPlayerController 0) "GrabHandClosed")
    (Variables|/Script/Engine.PostProcessVolume|SetbEnabled (Variables|/Game/TopDownBP/Blueprints/TopDownCharacter.TopDownCharacter_C|GetPostProcessVolumeEnemy (.AsTop%20Down%20Character (Utilities|Casting|CastToTopDownCharacter (Game|GetPlayerCharacter 0)))) true)
    (Rendering|SetRenderCustomDepth (Variables|Character|GetMesh) true)))

(event OnEndCursorOver(Mesh)
  (params (TouchedComponent :type Primitive%20Component%20Object%20Reference))
  (Variables|/Script/Engine.PlayerController|SetCurrentMouseCursor (Game|GetPlayerController 0) "Default")
  (Variables|/Script/Engine.PostProcessVolume|SetbEnabled (Variables|/Game/TopDownBP/Blueprints/TopDownCharacter.TopDownCharacter_C|GetPostProcessVolumeEnemy (.AsTop%20Down%20Character (Utilities|Casting|CastToTopDownCharacter (Game|GetPlayerCharacter 0)))) false)
  (Rendering|SetRenderCustomDepth (Variables|Character|GetMesh) false))

(event EventBeginPlay
  (|CallParentFunction) ; This node is disabled and will not be called.\nDrag off pins to build functionality.
)

(event Collision|EventActorBeginOverlap
  (params (OtherActor :type Actor%20Object%20Reference))
  (|CallParentFunction OtherActor) ; This node is disabled and will not be called.\nDrag off pins to build functionality.
)

(event EventTick
  (params (DeltaSeconds :type Float%20%28single-precision%29))
  (|CallParentFunction DeltaSeconds) ; This node is disabled and will not be called.\nDrag off pins to build functionality.
)

(fn ConstructionScript
  (|CallParentFunction))