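; Merchant NPC that the top-down character can trade with or rob.
; BeginPlay can roll the Offer from a data table by per-row chance, then converts it into storage items, stacking where allowed.
; Hovering highlights the merchant and picks the mode from Left Ctrl, while a sphere registers proximity.
; Interacting either opens the shop widget and freezes movement, or lazily spawns a chest of that stock, each gated by a DoOnce.
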(event OnComponentBeginOverlap(Sphere)
  (params (OverlappedComponent :type Primitive%20Component%20Object%20Reference) (OtherActor :type Actor%20Object%20Reference) (OtherComp :type Primitive%20Component%20Object%20Reference) (OtherBodyIndex :type Integer) (bFromSweep :type Boolean) (SweepResult :type Hit%20Result%20Structure%20%28by%20ref%29))
  (bind _astop_down_character (Utilities|Casting|CastToTopDownCharacter OtherActor))
  (Variables|/Game/TopDownBP/Blueprints/TopDownCharacter.TopDownCharacter_C|SetNearbyMerchant _astop_down_character self)
  (Rendering|SetVisibility (Variables|Default|GetMerchantText) true false))

(event OnComponentEndOverlap(Sphere)
  (params (OverlappedComponent :type Primitive%20Component%20Object%20Reference) (OtherActor :type Actor%20Object%20Reference) (OtherComp :type Primitive%20Component%20Object%20Reference) (OtherBodyIndex :type Integer))
  (bind _astop_down_character (Utilities|Casting|CastToTopDownCharacter OtherActor))
  (Variables|/Game/TopDownBP/Blueprints/TopDownCharacter.TopDownCharacter_C|SetNearbyMerchant _astop_down_character 0)
  (Rendering|SetVisibility (Variables|Default|GetMerchantText) false false))

(event OnBeginCursorOver(CapsuleComponent)
  (params (TouchedComponent :type Primitive%20Component%20Object%20Reference))
  (bind _astop_down_character (Utilities|Casting|CastToTopDownCharacter (Pawn|GetControlledPawn (Game|GetPlayerController 0))))
  (Variables|/Game/TopDownBP/Blueprints/TopDownCharacter.TopDownCharacter_C|SetMerchantCursor _astop_down_character self)
  (CallFunction|-SetCursor _astop_down_character)
  (Rendering|SetRenderCustomDepth (Variables|Character|GetMesh) true))

(event OnEndCursorOver(CapsuleComponent)
  (params (TouchedComponent :type Primitive%20Component%20Object%20Reference))
  (Variables|/Script/Engine.PlayerController|SetCurrentMouseCursor (Game|GetPlayerController 0) "Default")
  (bind _astop_down_character (Utilities|Casting|CastToTopDownCharacter (Pawn|GetControlledPawn (Game|GetPlayerController 0))))
  (Variables|/Game/TopDownBP/Blueprints/TopDownCharacter.TopDownCharacter_C|SetMerchantCursor _astop_down_character 0)
  (if (not (Variables|Default|GetisSelected?))
    (Rendering|SetRenderCustomDepth (Variables|Character|GetMesh) false)))

(event Custom|OnInteract
  (params (TopDownChar :type Top%20Down%20Character%20Object%20Reference))
  (bind _self self)
  (Variables|Default|SetTopDownChar TopDownChar)
  (if (not (Variables|Default|GetPlayerGrab?))
    ;[1 1 1] Совершаем покупку у продавца
    (Utilities|FlowControl|DoOnce false
      (:Completed
        (bind _returnvalue (UserInterface|CreateWidget "/Game/InventorySystem/Widgets/w_ShopWidget.w_ShopWidget_C" 0 self (Variables|Default|GetTopDownChar)))
        (Variables|Default|SetShopWidget _returnvalue)
        (Class|UserWidget|SetPositioninViewport :self (Variables|Default|GetShopWidget) :bRemoveDPIScale false)
        (Class|UserWidget|SetAnchorsinViewport (Variables|Default|GetShopWidget) (Utilities|Struct|MakeAnchors "(X=0.500000,Y=0.500000)" "(X=0.500000,Y=0.500000)"))
        (Class|UserWidget|SetAlignmentinViewport (Variables|Default|GetShopWidget) "(X=0.500000,Y=0.500000)")
        (UserInterface|Viewport|AddtoViewport (Variables|Default|GetShopWidget) 5)
        (Default|-HideInvetory (Variables|/Game/TopDownBP/Blueprints/TopDownCharacter.TopDownCharacter_C|GetInventoryRef (Variables|Default|GetTopDownChar)))
        (Default|-ShowInvetory (Variables|/Game/TopDownBP/Blueprints/TopDownCharacter.TopDownCharacter_C|GetInventoryRef (Variables|Default|GetTopDownChar)))
        (Variables|/Game/TopDownBP/Blueprints/TopDownCharacter.TopDownCharacter_C|SetIsShopOpen? (Variables|Default|GetTopDownChar) true)
        (Pawn|Components|CharacterMovement|DisableMovement (Variables|/Script/Engine.Character|GetCharacterMovement (Variables|Default|GetTopDownChar)))
        (Components|Movement|StopMovementImmediately (Variables|/Script/Engine.Character|GetCharacterMovement (Variables|Default|GetTopDownChar)))))
    (else
      ;[1 1 1] Грабим
      (Utilities|FlowControl|DoOnce false
        (:Completed
          (Variables|Default|GetStorageChest
            (:then
              _)
            (:else
              (bind _returnvalue_2 (Game|SpawnActorfromClass "/Game/InventorySystem/Blueprints/bp_Chest.bp_Chest_C" (Math|Transform|MakeTransform "0, 0, 0" "0, 0, 0" "1,1,1") "Undefined" _self 20 5 (Variables|Default|GetItemsStorage) false _self))
              (bind _output_get (Variables|Default|SetStorageChest _returnvalue_2))
              (Variables|/Game/InventorySystem/Blueprints/bp_Chest.bp_Chest_C|SetMerchant _output_get self)))
          (Default|OnInteract (Variables|Default|GetStorageChest) (Variables|Default|GetTopDownChar)))))))

(event Custom|OnShopClosed
  (bind _topdownchar (Variables|Default|GetTopDownChar))
  (bind _topdownchar_2 (Variables|Default|GetTopDownChar))
  (bind _inventoryref (Variables|/Game/TopDownBP/Blueprints/TopDownCharacter.TopDownCharacter_C|GetInventoryRef _topdownchar_2))
  (bind _charactermovement (Variables|/Script/Engine.Character|GetCharacterMovement _topdownchar_2))
  (bind _inventoryref_2 (Variables|/Game/TopDownBP/Blueprints/TopDownCharacter.TopDownCharacter_C|GetInventoryRef _topdownchar))
  (Variables|/Game/TopDownBP/Blueprints/TopDownCharacter.TopDownCharacter_C|SetIsShopOpen? _topdownchar false)
  (Pawn|Components|CharacterMovement|SetMovementMode (Variables|/Script/Engine.Character|GetCharacterMovement _topdownchar) "MOVE_Walking" 0)
  (if (Variables|/Game/InventorySystem/Blueprints/bp_Inventory.bp_Inventory_C|GetisVisible? _inventoryref_2)
    (Default|-HideInvetory _inventoryref_2)
    (Default|-ShowInvetory _inventoryref_2))
  (Widget|RemovefromParent (Variables|Default|GetShopWidget))
  (Variables|Default|SetShopWidget 0)
  ;[1 1 1] Совершаем покупку у продавца
  (Utilities|FlowControl|DoOnce false) ; enters at Reset
)

(event Custom|End_Rob
  (bind _self self)
  ;[1 1 1] Грабим
  (Utilities|FlowControl|DoOnce false) ; enters at Reset
)

(event EventBeginPlay
  (Utilities|FlowControl|Sequence
    (:then_0
      (if (Variables|Default|GetGenearteStartingItems?)
        (CallFunction|-GenerateStartingItems)))
    (:then_1
      (CallFunction|-GenerateStorageItems))))

(fn ConstructionScript)

(fn -GenerateStartingItems
  (bind _outrownames (DataTable|GetDataTableRowNames "/Game/InventorySystem/Blueprints/DataTables/Table_MerchantStarterItems.Table_MerchantStarterItems"))
  (for _array_element _outrownames
    (bind _returnvalue (Utilities|GetDataTableRow "/Game/InventorySystem/Blueprints/DataTables/Table_MerchantStarterItems.Table_MerchantStarterItems" _array_element)
      (:then
        (if (Math|Boolean|ANDBoolean (Utilities|IsValidClass (.ItemClass (Utilities|Struct|Breaks_MerchantContent _returnvalue))) (>= (.Chance (Utilities|Struct|Breaks_MerchantContent _returnvalue)) (Math|Random|RandomIntegerinRange 1 100)) true)
          (Utilities|Array|Add (Variables|Default|GetOffer) (.ItemClass (Utilities|Struct|Breaks_MerchantContent _returnvalue))))))))

(fn -SetCursor
  (params (Player :type Top%20Down%20Character%20Object%20Reference))
  (if (Variables|/Game/TopDownBP/Blueprints/TopDownCharacter.TopDownCharacter_C|GetLeftCtrl Player)
    (Variables|Default|SetPlayerGrab? true)
    (Variables|/Script/Engine.PlayerController|SetCurrentMouseCursor (Game|GetPlayerController 0) "GrabHandClosed")
    (else
      (Variables|Default|SetPlayerGrab? false)
      (Variables|/Script/Engine.PlayerController|SetCurrentMouseCursor (Game|GetPlayerController 0) "TextEditBeam"))))

(fn -GenerateStorageItems
  (for _array_element (Variables|Default|GetOffer)
    (Utilities|Array|Add (Variables|Default|GetItemsStorage) (Utilities|Struct|Makes_InventorySlot _array_element (Math|Integer|SelectInt 25 1 (.canBeStacked? (Utilities|Struct|Breaks_ItemInfo (.ItemInfo (Utilities|GetClassDefaults _array_element))))))))
  (return))

(fn -GenerateOffer
  (params (StartingItems :type Array%20of%20S%20Inventory%20Slot%20Structures))
  (bind _offer (Variables|Default|GetOffer))
  (Utilities|Array|Clear _offer)
  (for _array_element StartingItems
    (if (Utilities|IsValidClass (.ItemClass (Utilities|Struct|Breaks_InventorySlot _array_element)))
      (Utilities|Array|Add _offer (.ItemClass (Utilities|Struct|Breaks_InventorySlot _array_element)))))
  (return))